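; BP_Ball is a ball actor that moves in the XY plane and bounces off whatever blocks it.
; Each Tick it applies a swept world offset from Direction, Speed and delta time, with no physics simulation calls.
; On a blocking hit it reflects Direction about the surface normal and cuts Speed by a tenth, never dropping below MinSpeed.
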(event `self.ReceiveTick`
  (params (DeltaSeconds :type "Float (single-precision)"))
  (bind _returnvalue (* (`self.Speed`) 0.9))
  (bind (_returnvalue_x _returnvalue_y) (`KismetMathLibrary.BreakVector` (* (* (`self.Direction`) (`self.Speed`)) DeltaSeconds)))
  (bind _sweephitresult (`self.K2_AddActorWorldOffset` (`KismetMathLibrary.MakeVector` _returnvalue_x _returnvalue_y) true))
  (bind (_bblockinghit _binitialoverlap _time _distance _location _impactpoint _normal) (`GameplayStatics.BreakHitResult` _sweephitresult))
  (if _bblockinghit
    (set `self.Direction` (`KismetMathLibrary.GetReflectionVector` (`self.Direction`) _normal))
    (if (<= _returnvalue (`self.MinSpeed`))
      (set `self.Speed` (`self.MinSpeed`))
      (else
        (set `self.Speed` _returnvalue)))))

(fn `UserConstructionScript`)