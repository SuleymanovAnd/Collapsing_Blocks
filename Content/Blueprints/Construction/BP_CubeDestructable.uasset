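; BP_CubeDestructable is an actor, named as a destructible cube, that counts down a Life variable when other actors overlap it.
; Each overlap starts a 0.3 second Delay, which ignores re-triggers while pending, then decrements Life and prints it.
; When Life reaches exactly zero it calls the parent overlap event; the graph itself contains no destroy logic.
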(event `self.ReceiveActorBeginOverlap`
  (params (OtherActor :type "Actor Object Reference"))
  (bind _life (`self.life`))
  (`KismetSystemLibrary.Delay` 0.3)
  (set `self.life` (- _life 1))
  (`KismetSystemLibrary.PrintString` (`KismetStringLibrary.Conv_IntToString` _life) true true (struct :`R` 0.233602 :`G` 0.688264 :`B` 1.0 :`A` 1.0))
  (if (== 0 (`self.life`))
    (`parent.ReceiveActorBeginOverlap` OtherActor)))

(fn `UserConstructionScript`
  (`parent.UserConstructionScript`))